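; BP_helloActor is a practice actor whose Sphere component rolls back and forth along relative X.
; Tick moves and pitches the sphere by DeltaSeconds times Speed, flipping IsMoveRight at fixed limits either side of zero.
; BeginPlay prints the actor's display name, sets XValue and runs an empty loop.
; Disconnected experiments with XValue positioning, printing and basic operators remain unused in the graph.
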(event EventBeginPlay
  (Development|PrintString (Utilities|GetDisplayName self) true true "(R=0.437500,G=0.054579,B=0.384951,A=1.000000)" 1e+02)
  (Variables|Default|Setx%20value (+ 0.0 1.0))
  (for _index (range 0 5)
    _))

(event EventTick
  (params (DeltaSeconds :type Float%20%28single-precision%29))
  (bind _speed (Variables|Default|Getspeed))
  (bind _sphere (Variables|Default|GetSphere))
  (bind _speed_2 (Variables|Default|Getspeed))
  (bind _sphere_2 (Variables|Default|GetSphere))
  (bind _returnvalue (* DeltaSeconds _speed_2))
  (bind _returnvalue_2 (* DeltaSeconds _speed))
  (if (Variables|Default|Getis%20moveRight)
    ;[1 1 1] Right
    (Transformation|AddLocalRotation (Variables|Default|GetSphere) (Math|Rotator|MakeRotator 0.0 (* _returnvalue_2 -1.0) 0.0) false false)
    (Transformation|AddRelativeLocation _sphere_2 (Math|Vector|MakeVector _returnvalue_2 0.0 0.0) false false)
    (if (>= (.x (Variables|/Script/Engine.SceneComponent|GetRelativeLocation _sphere_2)) 1e+02)
      (Variables|Default|Setis%20moveRight false))
    (else
      ;[1 1 1] Left
      (Transformation|AddLocalRotation (Variables|Default|GetSphere) (Math|Rotator|MakeRotator 0.0 _returnvalue 0.0) false false)
      (Transformation|AddRelativeLocation _sphere (Math|Vector|MakeVector (* _returnvalue -1.0) 0.0 0.0) false false)
      (if (<= (.x (Variables|/Script/Engine.SceneComponent|GetRelativeLocation _sphere)) -1e+02)
        (Variables|Default|Setis%20moveRight true)))))

(fn ConstructionScript)